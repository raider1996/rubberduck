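; BP_KillZone is a kill volume that returns player cars to the start of the level.
; On BeginPlay it finds the BP_Start actor and caches its location.
; On overlap it casts to SportsCar_Pawn, falling back to SportsCar_Player2, then teleports that car to the cached location without sweep and calls its ResetEvent.
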(event `self.ReceiveBeginPlay`
  (bind _returnvalue (`GameplayStatics.GetActorOfClass` "/Game/BP_Start.BP_Start_C"))
  (set `self.Transform` (`self.K2_GetActorLocation` _returnvalue)))

(event `self.ReceiveActorBeginOverlap`
  (params (OtherActor :type "Actor Object Reference"))
  (bind _assports_car_pawn (cast `/Game/VehicleTemplate/Blueprints/SportsCar/SportsCar_Pawn` OtherActor)
    (:`then`
      (`self.K2_SetActorLocation` _assports_car_pawn (`self.Transform`) false true)
      (`/Game/VehicleTemplate/Blueprints/VehicleAdvPawn.resetEvent` _assports_car_pawn))
    (:`CastFailed`
      (bind _assports_car_player_2 (cast `/Game/VehicleTemplate/Blueprints/SportsCar/SportsCar_Player2` OtherActor))
      (`self.K2_SetActorLocation` _assports_car_player_2 (`self.Transform`) false true)
      (`/Game/VehicleTemplate/Blueprints/VehicleAdvPawn.resetEvent` _assports_car_player_2))))

(fn `UserConstructionScript`)