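; BP_BubblePickup is a car pickup that shows a temporary bubble screen when either of two player vehicles overlaps it.
; SportsCar_Pawn triggers the Player1 bubble widget and SportsCar_Player2 the Player2 one, each added to the viewport.
; The pickup then teleports far off the map instead of hiding, keeping it alive through a three-second delay before it removes the widget and destroys itself.
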(event `self.ReceiveActorBeginOverlap`
  (params (OtherActor :type "Actor Object Reference"))
  (cast `/Game/VehicleTemplate/Blueprints/SportsCar/SportsCar_Pawn` OtherActor
    (:`then`
      (bind _returnvalue (`|CreateWidget` "/Game/BPW_BubbleScreenPlayer1.BPW_BubbleScreenPlayer1_C"))
      (bind _output_get (set `self.Widget` _returnvalue))
      (`UserWidget.AddToViewport` _returnvalue 0)
      (`UserWidget.AddToViewport` _output_get 0))
    (:`CastFailed`
      (cast `/Game/VehicleTemplate/Blueprints/SportsCar/SportsCar_Player2` OtherActor)
      (bind _returnvalue_2 (`|CreateWidget` "/Game/BPW_BubbleScreenPlayer2.BPW_BubbleScreenPlayer2_C"))
      (bind _output_get_2 (set `self.Widget` _returnvalue_2))
      (`UserWidget.AddToViewport` _output_get_2 0)
      (`UserWidget.AddToViewport` _returnvalue_2 0)))
  (`self.K2_SetActorLocation` (-900000.0 -900000000.0 -900000000000.0)) ; teleport off map
  (`KismetSystemLibrary.Delay` 3.0)
  (`Widget.RemoveFromParent` (`self.Widget`))
  (`self.K2_DestroyActor`))

(fn `UserConstructionScript`)